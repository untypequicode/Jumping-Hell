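; BP_Box is a block with three trigger volumes, Up, Down and Dead, that react only to the BP_PJ pawn.
; Up calls SwitchUp and starts the pawn's timer, while Down calls SwitchDown and ends it.
; Outside menu mode, Up creates the death HUD and a forward delete timer, and Down creates the rebirth HUD and a reverse one.
; Dead calls Mort on the pawn.
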(event OnComponentBeginOverlap(Up)
  (params (OverlappedComponent :type Primitive%20Component%20Object%20Reference) (OtherActor :type Actor%20Object%20Reference) (OtherComp :type Primitive%20Component%20Object%20Reference) (OtherBodyIndex :type Integer) (bFromSweep :type Boolean) (SweepResult :type Hit%20Result%20Structure%20%28by%20ref%29))
  (bind _asbp_pj (Utilities|Casting|CastToBP_PJ OtherActor))
  (Default|SwitchUp _asbp_pj)
  (Default|StartTimer _asbp_pj)
  (if (not (Variables|/Game/BP/Personnages/PJ/BP_PJ.BP_PJ_C|GetIsMenu? _asbp_pj))
    (Default|CreateHUDDead _asbp_pj)
    (Default|Create/DeleteTimer _asbp_pj "Forward")))

(event OnComponentBeginOverlap(Down)
  (params (OverlappedComponent :type Primitive%20Component%20Object%20Reference) (OtherActor :type Actor%20Object%20Reference) (OtherComp :type Primitive%20Component%20Object%20Reference) (OtherBodyIndex :type Integer) (bFromSweep :type Boolean) (SweepResult :type Hit%20Result%20Structure%20%28by%20ref%29))
  (bind _asbp_pj (Utilities|Casting|CastToBP_PJ OtherActor))
  (Default|SwitchDown _asbp_pj)
  (Default|EndTimer _asbp_pj)
  (if (not (Variables|/Game/BP/Personnages/PJ/BP_PJ.BP_PJ_C|GetIsMenu? _asbp_pj))
    (Default|CreateHUDRebirth _asbp_pj)
    (Default|Create/DeleteTimer _asbp_pj "Reverse")))

(event OnComponentBeginOverlap(Dead)
  (params (OverlappedComponent :type Primitive%20Component%20Object%20Reference) (OtherActor :type Actor%20Object%20Reference) (OtherComp :type Primitive%20Component%20Object%20Reference) (OtherBodyIndex :type Integer) (bFromSweep :type Boolean) (SweepResult :type Hit%20Result%20Structure%20%28by%20ref%29))
  (bind _asbp_pj (Utilities|Casting|CastToBP_PJ OtherActor))
  (Default|Mort _asbp_pj))

(event EventBeginPlay)

(event Collision|EventActorBeginOverlap
  (params (OtherActor :type Actor%20Object%20Reference)))

(event EventTick
  (params (DeltaSeconds :type Float%20%28single-precision%29)))

(fn ConstructionScript)